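; BP_SS_GameMode is the game mode for the space shooter, tracking progress, kills and level, and starting a looping arcade track on BeginPlay.
; Tick adds ProgressIncrement to Progress every frame, without delta-time scaling.
; EnemyDestroyed counts kills and, because the count never resets here, raises Level on every kill from the third onward.
; PlayerDead forwards the death to BP_SS_HUD on the first player controller.
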(event `self.ReceiveBeginPlay`
  (`GameplayStatics.PlaySound2D` "/Game/00_SpaceShooter/Sounds/320995__littlerobotsoundfactory__loop_arcade_space_shooter_02.320995__littlerobotsoundfactory__loop_arcade_space_shooter_02" 1.0 1.0 0.0 null null))

(event `self.ReceiveTick`
  (params (DeltaSeconds :type "Float (single-precision)"))
  ;[1 1 1] Progress Increment
  (set `self.Progress` (+ (`self.Progress`) (`self.ProgressIncrement`))))

(event `PlayerDead`
  (bind _asbp_ss_hud (cast `/Game/00_SpaceShooter/BP_SS_HUD` (`PlayerController.GetHUD` (`GameplayStatics.GetPlayerController` 0))))
  (`/Game/00_SpaceShooter/BP_SS_HUD.PlayerDead` _asbp_ss_hud))

(event `EnemyDestroyed`
  (bind _output_get (set `self.EnemiesDestroyed` (+ (`self.EnemiesDestroyed`) 1)))
  (if (>= _output_get 3)
    (set `self.Level` (+ (`self.Level`) 1))))

(fn `UserConstructionScript`)