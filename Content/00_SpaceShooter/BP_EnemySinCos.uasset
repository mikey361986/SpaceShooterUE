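; Space shooter enemy Blueprint that moves in an oscillating sine or cosine pattern.
; Move offsets the actor in local space by Speed and DeltaTime, scaled by the sine or cosine of game time as IsSinOrCos selects.
; The wave follows the global clock rather than a per-actor timer, and movement does not sweep for collision.
; The event graph is inactive, and nothing here calls Move.
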(fn `Move`
  (params (DeltaTime :type "Float (double-precision)"))
  (bind _returnvalue (`GameplayStatics.GetTimeSeconds`))
  (bind _speed (`self.Speed`))
  (if (`self.IsSinOrCos`)
    (`self.K2_AddActorLocalOffset` (* (* (`KismetMathLibrary.Sin` _returnvalue) _speed) DeltaTime))
    (else
      (`self.K2_AddActorLocalOffset` (* (* _speed (`KismetMathLibrary.Cos` _returnvalue)) DeltaTime)))))

(fn `UserConstructionScript`
  (`parent.UserConstructionScript`))