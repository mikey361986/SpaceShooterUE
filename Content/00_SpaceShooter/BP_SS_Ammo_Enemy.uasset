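; BP_SS_Ammo_Enemy is the enemy projectile in the space shooter, exploding when it overlaps the player.
; On overlap it continues only for a BP_SS_Player without the "Limit" tag.
; It then prints the hit actor's name, spawns an explosion particle, plays a 2D sound and destroys itself after a short delay.
; The graph applies no damage and contains no movement logic.
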(event `self.ReceiveActorBeginOverlap`
  (params (OtherActor :type "Actor Object Reference"))
  ;[1 1 1] OnHit
  (cast `/Game/00_SpaceShooter/BP_SS_Player` OtherActor)
  (if (not (`KismetArrayLibrary.Array_Contains` (`Actor.Tags` OtherActor) "Limit"))
    (`KismetSystemLibrary.PrintString` (`KismetStringLibrary.Concat_StrStr` "Hit: " (`KismetSystemLibrary.GetObjectName` OtherActor)) true true (struct :`G` 1.0 :`B` 0.227797 :`A` 1.0))
    (`GameplayStatics.SpawnEmitterAtLocation` "/Game/StarterContent/Particles/P_Explosion.P_Explosion" (`self.K2_GetActorLocation`))
    (`GameplayStatics.PlaySound2D` "/Game/StarterContent/Audio/Explosion02.Explosion02" 1.0 1.0 0.0 null null)
    (`KismetSystemLibrary.Delay` 0.2)
    (`self.K2_DestroyActor`)))

(fn `UserConstructionScript`
  (`parent.UserConstructionScript`))