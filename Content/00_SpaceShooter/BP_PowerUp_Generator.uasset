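; Power-up spawner actor for the space shooter that periodically creates BP_PowerUp pickups.
; On BeginPlay it starts a looping timer at the SpawnTime interval and caches the BP_SS_GameMode reference, which the visible graphs never use.
; Each timer tick calls SpawnPowerUp, which spawns a power-up at the transform of a random scene component on itself tagged SpawnPointP.
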(event `self.ReceiveBeginPlay`
  (`KismetSystemLibrary.K2_SetTimerDelegate` (delegate `Spawn`) (`self.SpawnTime`) true)
  (bind _asbp_ss_game_mode (cast `/Game/00_SpaceShooter/BP_SS_GameMode` (`GameplayStatics.GetGameMode`)))
  (set `self.m_GameMode` _asbp_ss_game_mode))

(event `Spawn`
  (`self.SpawnPowerUp`))

(fn `SpawnPowerUp`
  (returns (PowerUpSpawned :type "/Game/00_SpaceShooter/BP_PowerUp Object Reference"))
  (bind _returnvalue (`self.GetComponentsByTag` "/Script/Engine.SceneComponent" "SpawnPointP"))
  (bind _returnvalue_2 (`|SpawnActorFromClass` "/Game/00_SpaceShooter/BP_PowerUp.BP_PowerUp_C" (`SceneComponent.K2_GetComponentToWorld` (`|GetArrayItem` _returnvalue (`KismetMathLibrary.RandomInteger` (`KismetArrayLibrary.Array_Length` _returnvalue)))) "Undefined" "MultiplyWithRoot" null null))
  (return _returnvalue_2))

(fn `UserConstructionScript`)