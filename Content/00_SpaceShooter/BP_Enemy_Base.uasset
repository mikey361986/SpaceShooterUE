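; Base enemy actor for the space shooter that flies straight along its starting forward vector and fires on a timer.
; Tick moves it without sweep and accumulates time to spawn an Ammo actor at FirePoint, facing the enemy's rotation.
; Overlapping an actor tagged Player or PowerUp calls its OnEnemyDestroy dispatcher for a delayed destroy, then notifies BP_SS_GameMode and refreshes the BP_SS_HUD widget.
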(event `self.ReceiveBeginPlay`
  (set `self.MovementVector` (`self.GetActorForwardVector`))
  (add `self.OnEnemyDestroy` (delegate `Destroyed_Event`)))

(event `Destroyed_Event`
  (`KismetSystemLibrary.Delay` 0.2)
  (`self.K2_DestroyActor`))

(event `self.ReceiveTick`
  (params (DeltaSeconds :type "Float (single-precision)"))
  (`self.Move` DeltaSeconds)
  (bind _output_get (set `self.ShotCurrentTime` (+ DeltaSeconds (`self.ShotCurrentTime`))))
  (if (>= _output_get (`self.DelayShoot`))
    (set `self.ShotCurrentTime` 0.0)
    (`self.Fire`)))

(event `self.ReceiveActorBeginOverlap`
  (params (OtherActor :type "Actor Object Reference"))
  (if (or (`KismetArrayLibrary.Array_Contains` (`Actor.Tags` OtherActor) "Player") (`KismetArrayLibrary.Array_Contains` (`Actor.Tags` OtherActor) "PowerUp"))
    (`KismetSystemLibrary.PrintString` "Enemy_base_Hit")
    (`self.OnEnemyDestroy`)
    (bind _asbp_ss_game_mode (cast `/Game/00_SpaceShooter/BP_SS_GameMode` (`GameplayStatics.GetGameMode`)))
    (`/Game/00_SpaceShooter/BP_SS_GameMode.EnemyDestroyed` _asbp_ss_game_mode)
    (bind _asbp_ss_hud (cast `/Game/00_SpaceShooter/BP_SS_HUD` (`PlayerController.GetHUD` (`GameplayStatics.GetPlayerController` 0))))
    (`/Game/00_SpaceShooter/BP_SS_HUD.UpdateWidget` _asbp_ss_hud)))

(fn `Fire`
  (bind _returnvalue (`|SpawnActorFromClass` (`self.Ammo`) (`SceneComponent.K2_GetComponentToWorld` (`self.FirePoint`)) "Undefined" "MultiplyWithRoot" null null))
  (`self.K2_SetActorRotation` _returnvalue (`self.K2_GetActorRotation`) false))

(fn `Move`
  (params (DeltaTime :type "Float (double-precision)"))
  (`self.K2_SetActorLocation` (+ (* (* DeltaTime (`self.Speed`)) (`self.MovementVector`)) (`self.K2_GetActorLocation`))))

(fn `UserConstructionScript`)