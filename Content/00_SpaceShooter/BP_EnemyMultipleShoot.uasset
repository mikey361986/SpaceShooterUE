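; Multi-shot enemy Blueprint for a space shooter that fires from two fire points at once.
; It overrides Fire, calls the parent implementation, then loops over both fire points to spawn an Ammo actor at each one's world transform and set its rotation to match.
; The event graph and construction script add no logic of their own, so all other behavior is left to the parent class.
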(fn `Fire`
  (`parent.Fire`)
  (bind _output_get (set `self.ArrayFirePoints` (`|MakeArray` (`self.FirePoint1`) (`self.FirePoint2`))))
  (for _array_element _output_get
    (bind _returnvalue (`|SpawnActorFromClass` (`self.Ammo`) (`SceneComponent.K2_GetComponentToWorld` _array_element) "Undefined" "MultiplyWithRoot" null null))
    (`self.K2_SetActorRotation` _returnvalue (`SceneComponent.K2_GetComponentRotation` _array_element) false)))

(fn `UserConstructionScript`
  (`parent.UserConstructionScript`))