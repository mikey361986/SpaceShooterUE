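; Player ship for the space shooter, handling movement, firing and lives.
; Enhanced Input stores the move axis, which Tick applies as an unswept location offset along the actor's right and forward vectors.
; Firing spawns Ammo at FirePoint with a laser sound, gated by a delay timer.
; Enemy-tagged overlaps or a debug key broadcast damage and remove a life, notifying BP_SS_GameMode when none remain.
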(event Custom|UpdateFire
  ;[1 1 1] Input Movement
  (Variables|Default|SetCanFire true))

(event Custom|DamageActor
  ;[1 1 1] Damage Player
  (Default|CallDamageActorDispatcher)
  (bind _output_get (Variables|Default|SetLives (- (Variables|Default|GetLives) 1)))
  (if (<= _output_get 0)
    (bind _output_get_2 (Variables|Default|SetLives 0))
    (bind _asbp_ss_game_mode (Utilities|Casting|CastToBP_SS_GameMode (Game|GetGameMode)))
    (Default|PlayerDead _asbp_ss_game_mode)
    (Variables|/Game/00_SpaceShooter/BP_SS_GameMode.BP_SS_GameMode_C|SetPlayerLives _asbp_ss_game_mode _output_get_2)))

(event Input|EnhancedActionEvents|EnhancedInputActionIA_Input_Fire
  (params (ActionValue :type Boolean) (ElapsedSeconds :type Float%20%28double-precision%29) (TriggeredSeconds :type Float%20%28double-precision%29) (InputAction :type Input%20Action%20Object%20Reference :default "/Game/00_SpaceShooter/IA_Input_Fire.IA_Input_Fire"))
  ;[1 1 1] Input Movement
  (:Triggered
    (if (Variables|Default|GetCanFire)
      (CallFunction|DoFire)
      (Variables|Default|SetCanFire false)
      (Utilities|Time|SetTimerbyEvent (delegate Custom|UpdateFire) (Variables|Default|GetFireDelay)))))

(event Input|EnhancedActionEvents|EnhancedInputActionIA_Input_Move
  (params (ActionValue :type Vector%202D%20Structure) (ElapsedSeconds :type Float%20%28double-precision%29) (TriggeredSeconds :type Float%20%28double-precision%29) (InputAction :type Input%20Action%20Object%20Reference :default "/Game/00_SpaceShooter/IA_Input_Move.IA_Input_Move"))
  ;[1 1 1] Input Movement
  (:Triggered
    (bind _output_get (Variables|Default|SetinputSaved ActionValue)))
  (:Canceled
    (Variables|Default|SetinputSaved "" :!label _label))
  (:Completed
    (goto _label)))

(event EventBeginPlay
  ;[1 1 1] Set Mapping Context
  (bind _asplayer_controller (Utilities|Casting|CastToPlayerController (Pawn|GetController)))
  (Utilities|IsValid (PlayerController|LocalPlayerSubsystems|GetEnhancedInputLocalPlayerSubsystem _asplayer_controller)
    (:Is%20Valid
      (Input|AddMappingContext (PlayerController|LocalPlayerSubsystems|GetEnhancedInputLocalPlayerSubsystem _asplayer_controller) "/Game/00_SpaceShooter/IMC_InputPlayer.IMC_InputPlayer" 0 "(bIgnoreAllPressedKeysUntilRelease=True,bForceImmediately=False)"))))

(event EventTick
  (params (DeltaSeconds :type Float%20%28single-precision%29))
  (bind _speed (Variables|Default|Getspeed))
  (bind _inputsaved (Variables|Default|GetinputSaved))
  (bind _returnvalue (* DeltaSeconds _speed))
  ;[1 1 1] Update Movement
  (Transformation|SetActorLocation (+ (+ (* (Transformation|GetActorRightVector) (* (.x _inputsaved) _returnvalue)) (* (* (.y _inputsaved) _returnvalue) (Transformation|GetActorForwardVector))) (Transformation|GetActorLocation)) false false))

(event Collision|EventActorBeginOverlap
  (params (OtherActor :type Actor%20Object%20Reference))
  ;[1 1 1] On Overlap Enemy
  (if (Utilities|Array|ContainsItem (Variables|/Script/Engine.Actor|GetTags OtherActor) "Enemy")
    (CallFunction|DamageActor)))

(event Input|KeyboardEvents|DebugKeyC
  (params (Key :type Key%20Structure :default "None") (ActionValue :type Input%20Action%20Value%20Structure))
  ;[1 1 1] Damage Player
  (:Pressed
    (CallFunction|DamageActor)))

(fn ConstructionScript)

(fn DoFire
  (Game|SpawnActorfromClass (Variables|Default|GetAmmo) (Transformation|GetWorldTransform (Variables|Default|GetFirePoint)) "Undefined" "MultiplyWithRoot" 0 0)
  (Audio|PlaySound2D "/Game/00_SpaceShooter/Sounds/519246__dukethedrake__lazer.519246__dukethedrake__lazer" 1.0 1.0 0.0 0 0))