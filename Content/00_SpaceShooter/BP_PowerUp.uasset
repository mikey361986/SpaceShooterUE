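; BP_PowerUp is a space shooter pickup that drifts in a random direction and destroys itself after its lifetime expires.
; BeginPlay picks a random yaw, which Tick applies while moving the actor forward by Speed.
; On overlap with a Player-tagged actor, it attaches to the player, emits sparks at the FirePoint and plays sounds.
; It also expands its sphere to a large radius, then destroys itself after a brief delay.
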(event `self.ReceiveBeginPlay`
  (`self.RandomRotation`)
  (`KismetSystemLibrary.Delay` (`self.LifeTime`))
  (`self.K2_DestroyActor`))

(event `self.ReceiveActorBeginOverlap`
  (params (OtherActor :type "Actor Object Reference"))
  (if (`KismetArrayLibrary.Array_Contains` (`Actor.Tags` OtherActor) "Player")
    (bind _asbp_ss_player (cast `/Game/00_SpaceShooter/BP_SS_Player` (`GameplayStatics.GetPlayerPawn` 0)))
    (bind _returnvalue (`GameplayStatics.SpawnEmitterAttached` "/Game/StarterContent/Particles/P_Sparks.P_Sparks" (`/Game/00_SpaceShooter/BP_SS_Player.FirePoint` _asbp_ss_player)))
    (set `self.Particle` _returnvalue)
    (`self.K2_AttachToActor` _asbp_ss_player "None" "SnapToTarget" "KeepRelative" "KeepRelative")
    (`SphereComponent.SetSphereRadius` (`self.Sphere`) 1000.0 true)
    (`GameplayStatics.PlaySound2D` "/Game/00_SpaceShooter/Sounds/503520__matrixxx__powerup-04.503520__matrixxx__powerup-04" 1.0 1.0 0.0 null null)
    (`GameplayStatics.PlaySound2D` "/Game/00_SpaceShooter/Sounds/506824__mrthenoronha__explosion-3-8-bit.506824__mrthenoronha__explosion-3-8-bit" 1.0 1.0 0.0 null null)
    (`KismetSystemLibrary.Delay` 0.2)
    (`ActorComponent.Deactivate` (`self.Particle`))
    (`KismetSystemLibrary.PrintString` (`KismetStringLibrary.Concat_StrStr` "Destroyed: " (`KismetSystemLibrary.GetDisplayName` self)))
    (set `self.Speed` 0.0)
    (`self.K2_DestroyActor`)))

(event `RandomRotation`
  (bind _rotation (`self.SetRandomRotation`)))

(event `self.ReceiveTick`
  (params (DeltaSeconds :type "Float (single-precision)"))
  (if (> (`self.Speed`) 0.0)
    (`self.K2_SetActorLocationAndRotation` (+ (* (* DeltaSeconds (`self.Speed`)) (`self.GetActorForwardVector`)) (`self.K2_GetActorLocation`)) (stale `RandomRotation` _rotation))))

(fn `SetRandomRotation`
  (returns (Rotation :type "Rotator Structure"))
  (bind (_returnvalue_roll _returnvalue_pitch) (`KismetMathLibrary.BreakRotator` (`self.K2_GetActorRotation`)))
  (bind _returnvalue (`KismetMathLibrary.MakeRotator` _returnvalue_roll _returnvalue_pitch (* 360.0 (`KismetMathLibrary.RandomFloat`))))
  (`KismetSystemLibrary.PrintString` (`KismetStringLibrary.Concat_StrStr` "Power UP Rotation: " (`KismetStringLibrary.Conv_RotatorToString` _returnvalue)))
  (return _returnvalue))

(fn `UserConstructionScript`)