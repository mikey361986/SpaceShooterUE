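; Enemy generator for the space shooter that spawns an enemy on a looping timer at a random SpawnPoint-tagged component.
; The GameMode's Level bounds a random pick among four enemy classes, clamped by MaxNumEnemies.
; SinCos enemies get a random wave flag, and only they reach the return node to get destroy events bound.
; Those events increase SpawnTime, but the running timer is never reset.
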(event `self.ReceiveBeginPlay`
  (`KismetSystemLibrary.K2_SetTimerDelegate` (delegate `Spawn`) (`self.SpawnTime`) true)
  (bind _asbp_ss_game_mode (cast `/Game/00_SpaceShooter/BP_SS_GameMode` (`GameplayStatics.GetGameMode`)))
  (set `self.m_GameMode` _asbp_ss_game_mode))

(event `Spawn`
  (bind _enemyspawned (`self.SpawnEnemy`))
  (bind _asbp_enemy_base (cast `/Game/00_SpaceShooter/BP_Enemy_Base` _enemyspawned))
  (add `/Game/00_SpaceShooter/BP_Enemy_Base.OnEnemyDestroy` _asbp_enemy_base (delegate `EnemyDestroyed`)))

(event `EnemyDestroyed`
  (set `self.SpawnTime` (+ (`self.SpawnTime`) 10.0)))

(fn `Get Class to Spawn`
  (params (Type :type Integer))
  (returns (Class :type "/Game/00_SpaceShooter/BP_Enemy_Base Class Reference"))
  (return (select `int` (`KismetMathLibrary.Clamp` Type 0 (- (`self.MaxNumEnemies`) 1)) :`0` "/Game/00_SpaceShooter/BP_Enemy_Base.BP_Enemy_Base_C" :`1` "/Game/00_SpaceShooter/BP_EnemyH.BP_EnemyH_C" :`2` "/Game/00_SpaceShooter/BP_EnemyMultipleShoot.BP_EnemyMultipleShoot_C" :`3` "/Game/00_SpaceShooter/BP_EnemySinCos.BP_EnemySinCos_C" :!type "/Game/00_SpaceShooter/BP_Enemy_Base Class Reference")))

(fn `SpawnEnemy`
  (returns (EnemySpawned :type "/Game/00_SpaceShooter/BP_Enemy_Base Object Reference"))
  (bind _returnvalue (`self.GetComponentsByTag` "/Script/Engine.SceneComponent" "SpawnPoint"))
  (bind _class (`self.Get Class to Spawn` (`KismetMathLibrary.RandomInteger` (`/Game/00_SpaceShooter/BP_SS_GameMode.Level` (`self.m_GameMode`)))))
  (bind _returnvalue_2 (`|SpawnActorFromClass` _class (`SceneComponent.K2_GetComponentToWorld` (`|GetArrayItem` _returnvalue (`KismetMathLibrary.RandomInteger` (`KismetArrayLibrary.Array_Length` _returnvalue)))) "Undefined" "MultiplyWithRoot" null null))
  ;[1 1 1] If only EnemySinCos
  (bind _asbp_enemy_sin_cos (cast `/Game/00_SpaceShooter/BP_EnemySinCos` _returnvalue_2))
  (set `/Game/00_SpaceShooter/BP_EnemySinCos.IsSinOrCos` (`KismetMathLibrary.RandomBool`) _asbp_enemy_sin_cos)
  (return _returnvalue_2))

(fn `UserConstructionScript`)