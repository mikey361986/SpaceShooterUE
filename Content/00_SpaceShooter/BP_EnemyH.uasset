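; BP_EnemyH is a space shooter enemy variant that sets a sideways movement direction and reverses it at side boundaries.
; On BeginPlay it sets MovementVector to the positive or negative actor right vector, based on IsRight.
; Overlapping an actor tagged "Side" toggles IsRight and negates MovementVector.
; The vector is not applied in this graph, and both events call their parent implementations first.
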(event `self.ReceiveBeginPlay`
  (bind _returnvalue (`self.GetActorRightVector`))
  ;[1 1 1] Setting Direction
  (`parent.ReceiveBeginPlay`)
  (if (`self.IsRight`)
    (set `self.MovementVector` (* _returnvalue 1))
    (else
      (set `self.MovementVector` (* _returnvalue -1)))))

(event `self.ReceiveActorBeginOverlap`
  (params (OtherActor :type "Actor Object Reference"))
  (`parent.ReceiveActorBeginOverlap` OtherActor)
  (if (`KismetArrayLibrary.Array_Contains` (`Actor.Tags` OtherActor) "Side")
    (if (`self.IsRight`)
      (set `self.IsRight` false)
      (else
        (set `self.IsRight` true)))
    (set `self.MovementVector` (* -1 (`self.MovementVector`)))))

(fn `UserConstructionScript`
  (`parent.UserConstructionScript`))