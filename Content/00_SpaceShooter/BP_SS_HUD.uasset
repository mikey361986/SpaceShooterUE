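; BP_SS_HUD is the Space Shooter HUD that puts the game widget on screen and feeds it player and match state.
; On BeginPlay it creates BP_SS_UserWidget, adds it to the viewport and caches the player character and game mode.
; It binds to the player's damage dispatcher instead of using Tick, pushing lives and enemies destroyed to the widget.
; A PlayerDead event forwards death to the widget.
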(event `self.ReceiveBeginPlay`
  (bind _returnvalue (`GameplayStatics.GetPlayerController` 0))
  ;[1 1 1] Show Widget to Player Controller
  (`/Engine/EditorBlueprintResources/StandardMacros.IsValid` _returnvalue
    (:`Is Valid`
      (bind _returnvalue_2 (`|CreateWidget` "/Game/00_SpaceShooter/BP_SS_UserWidget.BP_SS_UserWidget_C" _returnvalue))
      (bind _output_get (set `self.GameWidget` _returnvalue_2))
      (`UserWidget.AddToViewport` _output_get 0)
      (bind _asbp_ss_player (cast `/Game/00_SpaceShooter/BP_SS_Player` (`GameplayStatics.GetPlayerCharacter` 0)))
      (bind _output_get_2 (set `self.m_PlayerCharacter` _asbp_ss_player))
      (bind _asbp_ss_game_mode (cast `/Game/00_SpaceShooter/BP_SS_GameMode` (`GameplayStatics.GetGameMode`)))
      (set `self.m_GameMode` _asbp_ss_game_mode)
      ;[1 1 1] Event Dispatcher, create where is needed to call
      (add `/Game/00_SpaceShooter/BP_SS_Player.DamageActorDispatcher` _output_get_2 (delegate `UpdateWidget`)))))

(event `UpdateWidget`
  ;[1 1 1] Update Game Widget (User Widget)
  ;;[1 1 1] Before was Tick
  (`/Game/00_SpaceShooter/BP_SS_UserWidget.UpdateWidget` (`self.GameWidget`) (`/Game/00_SpaceShooter/BP_SS_Player.Lives` (`self.m_PlayerCharacter`)) (`/Game/00_SpaceShooter/BP_SS_GameMode.EnemiesDestroyed` (`self.m_GameMode`))))

(event `PlayerDead`
  (`/Game/00_SpaceShooter/BP_SS_UserWidget.PlayerDead` (`self.GameWidget`)))

(fn `UserConstructionScript`)